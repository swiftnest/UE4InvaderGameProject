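; Enemy actor for what appears to be an Invaders-style shooter, moving sideways, firing bullets and dying when hit by a player bullet.
; Tick moves it along Y using the shared DirectionY from MyGameState and counts down a randomized timer to spawn EnemyBulletBlueprint just below it.
; Overlapping a player bullet spawns an explosion, sends a score message to the game state and destroys the enemy.
; GetHealth and GetScore are stubs returning zero.
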(event `self.ReceiveBeginPlay`
  ;[1 1 1] 初期化
  (set `self.ShotTimer` (`KismetMathLibrary.RandomFloatInRange` 4.0 8.0)))

(event `self.ReceiveTick`
  (params (DeltaSeconds :type "Float (single-precision)"))
  (bind _returnvalue (- (`self.ShotTimer`) DeltaSeconds))
  ;[1 1 1] 左右移動
  (bind _asmygamestate_c (cast `/Game/Blueprints/MyGameState` (`GameplayStatics.GetGameState`)))
  (`self.K2_SetActorLocation` (+ (* (* (0.0 1.0 0.0) (`/Game/Blueprints/MyGameState.DirectionY` _asmygamestate_c)) (* (0.0 50.0 0.0) DeltaSeconds)) (`self.K2_GetActorLocation`)))
  (if (< _returnvalue 0.0)
    (`|SpawnActorFromClass` "/Game/Blueprints/EnemyBulletBlueprint.EnemyBulletBlueprint_C" (`KismetMathLibrary.Conv_VectorToTransform` (+ (`self.K2_GetActorLocation`) (0.0 0.0 -40.0))))
    (set `self.ShotTimer` (`KismetMathLibrary.RandomFloatInRange` 4.0 8.0))
    (else
      (set `self.ShotTimer` _returnvalue))))

(event `self.ReceiveActorBeginOverlap`
  (params (OtherActor :type "Actor Object Reference"))
  ;[1 1 1] 爆発
  (cast `/Game/Blueprints/PlayerBulletBlueprint` OtherActor)
  (`|SpawnActorFromClass` "/Game/Blueprints/Blueprint_Effect_ExplosionDummy.Blueprint_Effect_ExplosionDummy_C" (`KismetMathLibrary.Conv_VectorToTransform` (`self.K2_GetActorLocation`)))
  ;[1 1 1] スコア
  (message `/Game/Blueprints/MyInterface.AddScore` (`GameplayStatics.GetGameState`) 10)
  (`self.K2_DestroyActor`))

(fn `GetHealth`
  (returns (Health :type Integer))
  (return 0))

(fn `GetScore`
  (returns (Score :type Integer))
  (return 0))

(fn `UserConstructionScript`)