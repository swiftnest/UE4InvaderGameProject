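; Title screen HUD that draws the title image and handles its Start and End buttons.
; DrawHUD scales a 640x360 layout to screen width, centers it vertically and lays invisible hit boxes over the button areas.
; Clicks play a sound and, after a short delay, either quit or open the Invader level, replacing the hit boxes with a Now Loading image.
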(event `self.ReceiveDrawHUD`
  (params (SizeX :type Integer) (SizeY :type Integer))
  (bind _scale (`self.Scale`))
  (bind _returnvalue (* (`KismetMathLibrary.MakeVector2D` 250.0 58.0) (`self.Scale`)))
  (bind _returnvalue_2 (/ (- (`KismetMathLibrary.Conv_IntToDouble` SizeY) (* 360.0 _scale)) 2.0))
  (bind _returnvalue_3 (`KismetMathLibrary.MakeVector2D` 0.0 _returnvalue_2))
  (set `self.Scale` (/ (`KismetMathLibrary.Conv_IntToDouble` SizeX) 640.0))
  (`self.DrawTexture` "/Game/Textures/title.Title" 0.0 _returnvalue_2 640.0 360.0 0.0 0.0 1.0 1.0 (struct :`R` 1.0 :`G` 1.0 :`B` 1.0 :`A` 1.0) "BLEND_Opaque" _scale)
  (if (`self.IsLoading`)
    (`self.DrawTexture` "/Game/Textures/nowloading.nowloading" 0.0 0.0 320.0 64.0 0.0 0.0 1.0 1.0 (struct :`G` 0.216702 :`B` 1.0 :`A` 1.0) "BLEND_Translucent" (`self.Scale`))
    (else
      (`self.AddHitBox` (+ (* (`KismetMathLibrary.MakeVector2D` 23.0 214.0) (`self.Scale`)) _returnvalue_3) _returnvalue "Start")
      (`self.AddHitBox` (+ _returnvalue_3 (* (`KismetMathLibrary.MakeVector2D` 23.0 280.0) (`self.Scale`))) _returnvalue "End"))))

(event `self.ReceiveHitBoxClick`
  (params (BoxName :type Name))
  (`GameplayStatics.PlaySoundAtLocation` "/Game/Audio/ClickDummy.ClickDummy")
  (`KismetSystemLibrary.Delay` 1.0)
  (switch `name` BoxName
    (:`Start`
      (set `self.IsLoading` true)
      (`GameplayStatics.LoadStreamLevel` "Invader")
      (`GameplayStatics.OpenLevel` "Invader"))
    (:`End`
      (`KismetSystemLibrary.QuitGame` null))))

(fn `UserConstructionScript`)