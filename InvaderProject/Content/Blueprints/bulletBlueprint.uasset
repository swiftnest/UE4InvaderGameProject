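; Bullet projectile actor that deals fixed damage to any actor it overlaps, then destroys itself.
; MoveBullet offsets the bullet without sweeping, treating its Location input as a velocity scaled by DeltaTime, and destroys it outside a vertical Z range.
; The file has no Tick event or call to MoveBullet, so movement depends on an external caller.
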(event `self.ReceiveActorBeginOverlap`
  (params (OtherActor :type "Actor Object Reference"))
  (`GameplayStatics.ApplyDamage` OtherActor 10.0)
  (`self.K2_DestroyActor`))

(fn `MoveBullet`
  (params (Location :type "Object.Vector Structure") (DeltaTime :type "Float (double-precision)"))
  (bind _z (.z (`self.K2_GetActorLocation`)))
  (`self.K2_SetActorLocation` (+ (* Location DeltaTime) (`self.K2_GetActorLocation`)))
  (if (> _z 1000.0)
    (`self.K2_DestroyActor`)
    (elif (< _z -1000.0)
      (`self.K2_DestroyActor`))))

(fn `UserConstructionScript`)