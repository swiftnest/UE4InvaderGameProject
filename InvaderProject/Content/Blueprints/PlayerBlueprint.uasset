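; Player actor for a shooter that slides sideways along Y with the mouse, clamped to a fixed range.
; Left click spawns a bullet above the actor, or opens the Title level once the player is hidden after death.
; Damage plays a sound and lowers Health; at zero it spawns an explosion, then hides the actor and disables its collision.
; GetHealth exposes Health, while GetScore is a stub that always returns zero.
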(event `InputAxisKey|MouseX`
  (params (AxisValue :type "Float (single-precision)"))
  ;[1 1 1] 移動
  (`self.K2_SetActorLocation` (`KismetMathLibrary.MakeVector` (.x (+ (* (0.0 30.0 0.0) AxisValue) (`self.K2_GetActorLocation`))) (`KismetMathLibrary.FMin` (`KismetMathLibrary.FMax` (.y (+ (* (0.0 30.0 0.0) AxisValue) (`self.K2_GetActorLocation`))) -400.0) 400.0) (.z (+ (* (0.0 30.0 0.0) AxisValue) (`self.K2_GetActorLocation`))))))

(event `Key|LeftMouseButton`
  ;[1 1 1] 弾の発射
  (:`Pressed`
    (if (`self.bHidden`)
      (`GameplayStatics.OpenLevel` "Title")
      (else
        (`|SpawnActorFromClass` "/Game/Blueprints/PlayerBulletBlueprint.PlayerbulletBlueprint_C" (`KismetMathLibrary.Conv_VectorToTransform` (+ (`self.K2_GetActorLocation`) (0.0 0.0 50.0))))))))

(event `self.ReceiveAnyDamage`
  (params (Damage :type "Float (single-precision)") (DamageType :type "DamageType Object Reference") (InstigatedBy :type "Controller Object Reference") (DamageCauser :type "Actor Object Reference"))
  ;[1 1 1] ダメージ処理
  (`GameplayStatics.PlaySoundAtLocation` "/Game/Audio/ShotDummy.ShotDummy" (`self.K2_GetActorLocation`))
  (set `self.Health` (- (`self.Health`) (`KismetMathLibrary.FFloor` Damage)))
  ;[1 1 1] 死亡処理
  (if (<= (`self.Health`) 0)
    (`|SpawnActorFromClass` "/Game/Blueprints/Blueprint_Effect_ExplosionDummy.Blueprint_Effect_ExplosionDummy_C" (`KismetMathLibrary.Conv_VectorToTransform` (`self.K2_GetActorLocation`)))
    (`self.SetActorHiddenInGame` true)
    (`self.SetActorEnableCollision` false)))

(fn `GetHealth`
  (returns (Health :type Integer))
  (return (`self.Health`)))

(fn `GetScore`
  (returns (Score :type Integer))
  (return 0))

(fn `UserConstructionScript`)